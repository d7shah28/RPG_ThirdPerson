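; Player stats component that tracks health, stamina, XP and level for BP_Player.
; Increase and decrease functions change the values and immediately push bars and text to the player's HUD widget, with a first refresh one tick after BeginPlay.
; Decrease functions report depletion, and reaching max XP raises the level, resets XP and raises the next threshold.
; Stamina overflow in IncreaseStamina sets CurrentHealth to MaxStamina rather than capping stamina.
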(event `self.ReceiveBeginPlay`
  (`|ExecutionSequence`
    (:`then_0`
      (bind _asbp_player (cast `/Game/Blueprints/Player/BP_Player` (`self.GetOwner`)))
      (set `self.PlayerReference` _asbp_player))
    (:`then_1`
      (`KismetSystemLibrary.DelayUntilNextTick`)
      (`self.UpdateStaminaBar`)
      (`self.UpdateHealthBar`)
      (`self.UpdateLevelXpBar`))))

(fn `DecreaseHealth`
  (params (Damage :type "Float (double-precision)"))
  (returns (`isPlayerDead?` :type Boolean))
  (if (not (<= (`self.CurrentHealth`) 0.0))
    (set `self.CurrentHealth` (- (`self.CurrentHealth`) Damage))
    (`self.UpdateHealthBar`)
    (if (<= (`self.CurrentHealth`) 0.0)
      (return true)
      (else
        (return false)))))

(fn `DecreaseStamina`
  (params (DepletedStamina :type "Float (double-precision)"))
  (returns (`StaminaDepleted?` :type Boolean))
  (if (not (<= (`self.CurrentStamina`) 0.0))
    (set `self.CurrentStamina` (- (`self.CurrentStamina`) DepletedStamina))
    (`self.UpdateStaminaBar`)
    (if (<= (`self.CurrentStamina`) 0.0)
      (return true)
      (else
        (return false)))))

(fn `IncreaseHealth`
  (params (A :type "Float (double-precision)"))
  (bind _output_get (set `self.CurrentHealth` (+ A (`self.CurrentHealth`))))
  (if (> _output_get (`self.MaxHealth`))
    (set `self.CurrentHealth` (`self.MaxHealth`)))
  (`self.UpdateHealthBar`))

(fn `IncreaseLevel`
  (params (AddedLevel :type Integer))
  (set `self.Level` (+ AddedLevel (`self.Level`)))
  (set `self.MaxXp` (+ 150.0 (`self.MaxXp`)))
  (set `self.Xp` 0.0)
  (`self.UpdateLevelXpBar`))

(fn `IncreaseMaxHealth`
  (params (Incremention :type "Float (double-precision)"))
  (set `self.MaxHealth` (+ Incremention (`self.MaxHealth`)))
  (`self.UpdateHealthBar`))

(fn `IncreaseMaxStamina`
  (params (AddedStamina :type "Float (double-precision)"))
  (set `self.MaxStamina` (+ AddedStamina (`self.MaxStamina`)))
  (`self.UpdateStaminaBar`))

(fn `IncreaseStamina`
  (params (AddedStamina :type "Float (double-precision)"))
  (bind _output_get (set `self.CurrentStamina` (+ AddedStamina (`self.CurrentStamina`))))
  (if (> _output_get (`self.MaxStamina`))
    (set `self.CurrentHealth` (`self.MaxStamina`)))
  (`self.UpdateStaminaBar`))

(fn `IncreaseXP`
  (params (Xp :type "Float (double-precision)"))
  (bind _output_get (set `self.Xp` (+ Xp (`self.Xp`))))
  (`self.UpdateLevelXpBar`)
  (if (>= _output_get (`self.MaxXp`))
    (`self.IncreaseLevel` 1)))

(fn `UpdateHealthBar`
  (bind _returnvalue (/ (`self.CurrentHealth`) (`self.MaxHealth`)))
  (bind _hudwidgetreference (`/Game/Blueprints/Player/BP_Player.HudWidgetReference` (`self.PlayerReference`)))
  (`ProgressBar.SetPercent` (`/Game/UI/WBP_Hud.HealthBar` _hudwidgetreference) _returnvalue)
  (`TextBlock.SetText` (`/Game/UI/WBP_Hud.T_Health` _hudwidgetreference) (`KismetTextLibrary.Conv_DoubleToText` (* _returnvalue 100.0) "HalfToEven")))

(fn `UpdateLevelXpBar`
  (bind _hudwidgetreference (`/Game/Blueprints/Player/BP_Player.HudWidgetReference` (`self.PlayerReference`)))
  (`ProgressBar.SetPercent` (`/Game/UI/WBP_Hud.XpBar` _hudwidgetreference) (/ (`self.Xp`) (`self.MaxXp`)))
  (`TextBlock.SetText` (`/Game/UI/WBP_Hud.T_Xp` _hudwidgetreference) (`|FormatText` "{CurrentXP}/{MaxHp}" (`self.Xp`) (`self.MaxXp`)))
  (`TextBlock.SetText` (`/Game/UI/WBP_Hud.T_PlayerLevel` _hudwidgetreference) (`KismetTextLibrary.Conv_IntToText` (`self.Level`))))

(fn `UpdateStaminaBar`
  (`ProgressBar.SetPercent` (`/Game/UI/WBP_Hud.StaminaBar` (`/Game/Blueprints/Player/BP_Player.HudWidgetReference` (`self.PlayerReference`))) (/ (`self.CurrentStamina`) (`self.MaxStamina`))))