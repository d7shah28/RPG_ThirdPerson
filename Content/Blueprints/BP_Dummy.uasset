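; Target dummy for back stealth assassinations with a paired knife animation.
; An overlap radius shows the assassinate widget while BP_Player is inside.
; StealthBackAssassin plays the victim montage, hides the widget, starts Ragdoll and returns the AssassinRef location and dummy rotation for placing the attacker.
; Ragdoll uses parallel fixed delays to play the death sound, then enable mesh physics, rather than montage notifies.
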(event `Ragdoll`
  (`|ExecutionSequence`
    (:`then_0`
      (`KismetSystemLibrary.Delay` 2.5)
      (`PrimitiveComponent.SetSimulatePhysics` (`self.Mesh`) true))
    (:`then_1`
      (`KismetSystemLibrary.Delay` 1.7)
      (`GameplayStatics.PlaySoundAtLocation` "/Game/Audio/Grunts-Hits/SC_Death.SC_Death" (`self.K2_GetActorLocation`) (struct) 1.0 1.0 0.0 null null null null))))

(event `self.AssasinationRadius.OnComponentBeginOverlap`
  (params (OverlappedComponent :type "PrimitiveComponent Object Reference") (OtherActor :type "Actor Object Reference") (OtherComp :type "PrimitiveComponent Object Reference") (OtherBodyIndex :type Integer) (bFromSweep :type Boolean) (SweepResult :type "HitResult Structure (by ref)"))
  (cast `/Game/Blueprints/Player/BP_Player` OtherActor)
  (`SceneComponent.SetVisibility` (`self.AssassinateWidget`) true false))

(event `self.AssasinationRadius.OnComponentEndOverlap`
  (params (OverlappedComponent :type "PrimitiveComponent Object Reference") (OtherActor :type "Actor Object Reference") (OtherComp :type "PrimitiveComponent Object Reference") (OtherBodyIndex :type Integer))
  (cast `/Game/Blueprints/Player/BP_Player` OtherActor)
  (`SceneComponent.SetVisibility` (`self.AssassinateWidget`) false false))

(fn `StealthBackAssassin`
  (returns (ReferenceLocation :type "Vector Structure") (`Assassin Rotation` :type "Rotator Structure"))
  (`self.PlayAnimMontage` "/Game/RPG_Character/Animations/Assasinations/Paired_Knife_Stealth_KidneyAndNeck_Vic_Montage.Paired_Knife_Stealth_KidneyAndNeck_Vic_Montage")
  (`SceneComponent.SetVisibility` (`self.AssassinateWidget`) false false)
  (`self.Ragdoll`)
  (return (`SceneComponent.K2_GetComponentLocation` (`self.AssassinRef`)) (`self.K2_GetActorRotation`)))

(fn `UserConstructionScript`)